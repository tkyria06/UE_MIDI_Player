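; Drum kit Blueprint that lights up its pieces in response to MIDI notes from a MetaSound.
; On BeginPlay it adds an audio component and watches its "MIDI Stream" output through the MetaSound Output Subsystem.
; Each event's note number selects a drum or cymbal, whose meshes swap to a glow material for a brief Delay, then revert.
; The SetMaterialDrums helper is left unused.
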(event `self.ReceiveBeginPlay`
  (bind _returnvalue (`AddComponent|NODE_AddAudioComponent-2`))
  (`MetaSoundOutputSubsystem.WatchOutput` (subsystem `MetaSoundOutputSubsystem`) _returnvalue "MIDI Stream" (delegate `MidiStream`) "None" "None"))

(event `MidiStream`
  (params (OutputName :type Name) (Output :type "MetaSoundOutput Structure (by ref)"))
  (bind _drumset_bass_pedal (`self.DrumSet_Bass_Pedal`))
  (bind _drumset_cymbal_hihat (`self.DrumSet_Cymbal_HiHat`))
  (bind _drumset_cymbal_ride (`self.DrumSet_Cymbal_Ride`))
  (bind _drumset_bass (`self.DrumSet_Bass`))
  (bind _drumset_snare (`self.DrumSet_Snare`))
  (bind _drumset_tom_floor (`self.DrumSet_Tom_Floor`))
  (bind _drumset_tom_mid (`self.DrumSet_Tom_Mid`))
  (bind _drumset_tom_high (`self.DrumSet_Tom_High`))
  (bind _drumset_cymbal_crash (`self.DrumSet_Cymbal_Crash`))
  ;[1 1 1] Get Active Drums Notes (might be note on/ note off)
  (bind (_success _returnvalue) (`MidiEventInfoBlueprintLibrary.GetMidiEventInfo` Output))
  (bind _returnvalue_2 (`MidiEventInfoBlueprintLibrary.GetNoteNumber` _returnvalue))
  (switch `string` (`KismetTextLibrary.Conv_TextToString` (`KismetTextLibrary.Conv_StringToText` (`KismetStringLibrary.Conv_IntToString` _returnvalue_2)))
    (:`36`
      (`PrimitiveComponent.SetMaterial` _drumset_bass 0 "/Game/Keys/Materials/White_Glow.White_Glow")
      (`PrimitiveComponent.SetMaterial` _drumset_bass_pedal 0 "/Game/Keys/Materials/White_Glow.White_Glow")
      (`PrimitiveComponent.SetMaterial` (`self.DrumSet_Lid_004`) 0 "/Game/Keys/Materials/White_Glow.White_Glow")
      (`KismetSystemLibrary.Delay` 0.1)
      (`PrimitiveComponent.SetMaterial` _drumset_bass 0 "/Game/Keys/Materials/White.White")
      (`PrimitiveComponent.SetMaterial` _drumset_bass_pedal 0 "/Game/Drums/DrumSet.DrumSet")
      (`PrimitiveComponent.SetMaterial` (`self.DrumSet_Lid_004`) 0 "/Game/Drums/DrumSet.DrumSet"))
    (:`38`
      (`PrimitiveComponent.SetMaterial` _drumset_snare 0 "/Game/Keys/Materials/White_Glow.White_Glow")
      (`PrimitiveComponent.SetMaterial` (`self.DrumSet_Lid_003`) 0 "/Game/Keys/Materials/White_Glow.White_Glow")
      (`KismetSystemLibrary.Delay` 0.1)
      (`PrimitiveComponent.SetMaterial` _drumset_snare 0 "/Game/Keys/Materials/White.White")
      (`PrimitiveComponent.SetMaterial` (`self.DrumSet_Lid_003`) 0 "/Game/Drums/DrumSet.DrumSet"))
    (:`43`
      (`PrimitiveComponent.SetMaterial` _drumset_tom_floor 0 "/Game/Keys/Materials/White_Glow.White_Glow")
      (`PrimitiveComponent.SetMaterial` (`self.DrumSet_Lid`) 0 "/Game/Keys/Materials/White_Glow.White_Glow")
      (`KismetSystemLibrary.Delay` 0.1)
      (`PrimitiveComponent.SetMaterial` _drumset_tom_floor 0 "/Game/Keys/Materials/White.White")
      (`PrimitiveComponent.SetMaterial` (`self.DrumSet_Lid`) 0 "/Game/Drums/DrumSet.DrumSet"))
    (:`45`
      (`PrimitiveComponent.SetMaterial` _drumset_tom_mid 0 "/Game/Keys/Materials/White_Glow.White_Glow")
      (`PrimitiveComponent.SetMaterial` (`self.DrumSet_Lid_001`) 0 "/Game/Keys/Materials/White_Glow.White_Glow")
      (`KismetSystemLibrary.Delay` 0.1)
      (`PrimitiveComponent.SetMaterial` _drumset_tom_mid 0 "/Game/Keys/Materials/White.White")
      (`PrimitiveComponent.SetMaterial` (`self.DrumSet_Lid_001`) 0 "/Game/Drums/DrumSet.DrumSet"))
    (:`48`
      (`PrimitiveComponent.SetMaterial` _drumset_tom_high 0 "/Game/Keys/Materials/White_Glow.White_Glow")
      (`PrimitiveComponent.SetMaterial` (`self.DrumSet_Lid_002`) 0 "/Game/Keys/Materials/White_Glow.White_Glow")
      (`KismetSystemLibrary.Delay` 0.1)
      (`PrimitiveComponent.SetMaterial` _drumset_tom_high 0 "/Game/Keys/Materials/White.White")
      (`PrimitiveComponent.SetMaterial` (`self.DrumSet_Lid_002`) 0 "/Game/Drums/DrumSet.DrumSet"))
    (:`49`
      (`PrimitiveComponent.SetMaterial` _drumset_cymbal_crash 0 "/Game/Keys/Materials/Black_Glow.Black_Glow")
      (`KismetSystemLibrary.Delay` 0.1)
      (`PrimitiveComponent.SetMaterial` _drumset_cymbal_crash 0 "/Game/StarterContent/Materials/M_Metal_Gold.M_Metal_Gold"))
    (:`42`
      (`PrimitiveComponent.SetMaterial` _drumset_cymbal_hihat 0 "/Game/Keys/Materials/Black_Glow.Black_Glow")
      (`KismetSystemLibrary.Delay` 0.1)
      (`PrimitiveComponent.SetMaterial` _drumset_cymbal_hihat 0 "/Game/StarterContent/Materials/M_Metal_Gold.M_Metal_Gold"))
    (:`51`
      (`PrimitiveComponent.SetMaterial` _drumset_cymbal_ride 0 "/Game/Keys/Materials/Black_Glow.Black_Glow")
      (`KismetSystemLibrary.Delay` 0.1)
      (`PrimitiveComponent.SetMaterial` _drumset_cymbal_ride 0 "/Game/StarterContent/Materials/M_Metal_Gold.M_Metal_Gold"))))

(fn `SetMaterialDrums`
  (params (DrumsComponent :type "StaticMeshComponent Object Reference"))
  (`PrimitiveComponent.SetMaterial` DrumsComponent 0 "/Game/Keys/Materials/Black_Glow.Black_Glow"))

(fn `UserConstructionScript`)