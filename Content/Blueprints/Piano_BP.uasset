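; Piano Blueprint that animates and lights its 88 keys in response to MIDI events from a MetaSound.
; BeginPlay builds the key array, adds an audio component and watches its "MIDI Stream" output.
; Each note, offset by 21, toggles KeyPlaying to press or reset that key, inferring note on/off rather than reading the event type.
; SetGlow picks white or black glow materials by checking the current material's name.
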(event `self.ReceiveBeginPlay`
  (`self.MakePianoKeysArray`)
  (bind _returnvalue (`AddComponent|NODE_AddAudioComponent-0`))
  (`MetaSoundOutputSubsystem.WatchOutput` (subsystem `MetaSoundOutputSubsystem`) _returnvalue "MIDI Stream" (delegate `MidiStream`) "None" "None"))

(event `MidiStream`
  (params (OutputName :type Name) (Output :type "MetaSoundOutput Structure (by ref)"))
  ;[1 1 1] Get Active Piano Notes (might be note on/ note off)
  (bind (_success _returnvalue) (`MidiEventInfoBlueprintLibrary.GetMidiEventInfo` Output))
  (bind _returnvalue_2 (`MidiEventInfoBlueprintLibrary.GetNoteNumber` _returnvalue))
  (if (> _returnvalue_2 0)
    (bind _returnvalue_3 (- _returnvalue_2 21))
    (if (`|GetArrayItem` (`self.KeyPlaying`) _returnvalue_3)
      ;[1 0 0] If note is already playing, then its a note off and reset the transform of the key
      (`self.SetKeyTransform` _returnvalue_3 (`KismetMathLibrary.MakeTransform` (0.0 0.0 0.0)))
      (`self.SetGlow` false _returnvalue_3)
      (else
        ;[0 1 0] If note did not played, then its a note on and make the transformation of the key
        (`self.SetKeyTransform` _returnvalue_3 (`KismetMathLibrary.MakeTransform` (0.0 0.0 -2.0) (struct :`Roll` 6.0)) true)
        (`self.SetGlow` true _returnvalue_3)))))

(fn `MakePianoKeysArray`
  (set `self.Piano_Keys` (`|MakeArray` (`self.Keys_PianoKey_001`) (`self.Keys_PianoKey_002`) (`self.Keys_PianoKey_003`) (`self.Keys_PianoKey_004`) (`self.Keys_PianoKey_005`) (`self.Keys_PianoKey_006`) (`self.Keys_PianoKey_007`) (`self.Keys_PianoKey_008`) (`self.Keys_PianoKey_009`) (`self.Keys_PianoKey_010`) (`self.Keys_PianoKey_011`) (`self.Keys_PianoKey_012`) (`self.Keys_PianoKey_013`) (`self.Keys_PianoKey_014`) (`self.Keys_PianoKey_015`) (`self.Keys_PianoKey_016`) (`self.Keys_PianoKey_017`) (`self.Keys_PianoKey_018`) (`self.Keys_PianoKey_019`) (`self.Keys_PianoKey_020`) (`self.Keys_PianoKey_021`) (`self.Keys_PianoKey_022`) (`self.Keys_PianoKey_023`) (`self.Keys_PianoKey_024`) (`self.Keys_PianoKey_025`) (`self.Keys_PianoKey_026`) (`self.Keys_PianoKey_027`) (`self.Keys_PianoKey_028`) (`self.Keys_PianoKey_029`) (`self.Keys_PianoKey_030`) (`self.Keys_PianoKey_031`) (`self.Keys_PianoKey_032`) (`self.Keys_PianoKey_033`) (`self.Keys_PianoKey_034`) (`self.Keys_PianoKey_035`) (`self.Keys_PianoKey_036`) (`self.Keys_PianoKey_037`) (`self.Keys_PianoKey_038`) (`self.Keys_PianoKey_039`) (`self.Keys_PianoKey_040`) (`self.Keys_PianoKey_041`) (`self.Keys_PianoKey_042`) (`self.Keys_PianoKey_043`) (`self.Keys_PianoKey_044`) (`self.Keys_PianoKey_045`) (`self.Keys_PianoKey_046`) (`self.Keys_PianoKey_047`) (`self.Keys_PianoKey_048`) (`self.Keys_PianoKey_049`) (`self.Keys_PianoKey_050`) (`self.Keys_PianoKey_051`) (`self.Keys_PianoKey_052`) (`self.Keys_PianoKey_053`) (`self.Keys_PianoKey_054`) (`self.Keys_PianoKey_055`) (`self.Keys_PianoKey_056`) (`self.Keys_PianoKey_057`) (`self.Keys_PianoKey_058`) (`self.Keys_PianoKey_059`) (`self.Keys_PianoKey_060`) (`self.Keys_PianoKey_061`) (`self.Keys_PianoKey_062`) (`self.Keys_PianoKey_063`) (`self.Keys_PianoKey_064`) (`self.Keys_PianoKey_065`) (`self.Keys_PianoKey_066`) (`self.Keys_PianoKey_067`) (`self.Keys_PianoKey_068`) (`self.Keys_PianoKey_069`) (`self.Keys_PianoKey_070`) (`self.Keys_PianoKey_071`) (`self.Keys_PianoKey_072`) (`self.Keys_PianoKey_073`) (`self.Keys_PianoKey_074`) (`self.Keys_PianoKey_075`) (`self.Keys_PianoKey_076`) (`self.Keys_PianoKey_077`) (`self.Keys_PianoKey_078`) (`self.Keys_PianoKey_079`) (`self.Keys_PianoKey_080`) (`self.Keys_PianoKey_081`) (`self.Keys_PianoKey_082`) (`self.Keys_PianoKey_083`) (`self.Keys_PianoKey_084`) (`self.Keys_PianoKey_085`) (`self.Keys_PianoKey_086`) (`self.Keys_PianoKey_087`) (`self.Keys_PianoKey_088`) :!type "MeshComponent Object Reference")))

(fn `SetGlow`
  (params (Glow :type Boolean) (Index :type Integer))
  (bind _output (`|GetArrayItem` (`self.Piano_Keys`) Index))
  (if (`KismetStringLibrary.Contains` (`KismetSystemLibrary.GetDisplayName` (`PrimitiveComponent.GetMaterial` _output 0)) "White")
    (if Glow
      (`PrimitiveComponent.SetMaterial` _output 0 "/Game/Keys/Materials/White_Glow.White_Glow")
      (else
        (`PrimitiveComponent.SetMaterial` _output 0 "/Game/Keys/Materials/White.White")))
    (elif Glow
      (`PrimitiveComponent.SetMaterial` _output 0 "/Game/Keys/Materials/Black_Glow.Black_Glow")
      (else
        (`PrimitiveComponent.SetMaterial` _output 0 "/Game/Keys/Materials/Black.Black")))))

(fn `SetKeyTransform`
  (params (Index :type Integer) (Transform :type "Transform Structure") (SetPlayingTrue :type Boolean))
  (`SceneComponent.K2_SetRelativeTransform` (`|GetArrayItem` (`self.Piano_Keys`) Index) (`KismetMathLibrary.MakeTransform` Transform_Location Transform_Rotation) false false)
  (`KismetArrayLibrary.Array_Set` (`self.KeyPlaying`) Index SetPlayingTrue))

(fn `UserConstructionScript`)